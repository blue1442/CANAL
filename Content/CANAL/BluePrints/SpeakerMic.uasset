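; SpeakerMic is an interactable microphone that shows a boat color widget when the Game Instance reports a boat on the sea.
; On interaction it stores the boat's color as text, lights a material and displays the BoatColor UI with a randomized Time.
; After a separately randomized delay it removes the widget and switches the light off, with an InProgress flag blocking repeat use meanwhile.
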(event EventBeginPlay
  (bind _asgame_instance (Utilities|Casting|CastToGame_Instance (Game|GetGameInstance)))
  (Variables|Default|SetGame%20Instance _asgame_instance))

(event EventInteractwithObject
  (bind _returnvalue (Math|Random|RandomIntegerinRange 4 8))
  (bind _game_instance (Variables|Default|GetGame%20Instance))
  (if (and (== (Variables|Default|GetInProgress) false) (Variables|/Game/CANAL/BluePrints/Game_Instance.Game_Instance_C|GetBoatOnSea _game_instance))
    (Development|PrintString "Getting boat color")
    (Variables|Default|SetTextColor (Utilities|Text|ToText(String) (Variables|/Game/CANAL/BluePrints/Game_Instance.Game_Instance_C|GetBoatColor _game_instance)))
    (Rendering|Material|SetScalarParameterValueonMaterials (Variables|Default|GetLight1) "Light" 2.0)
    (bind _returnvalue_2 (UserInterface|CreateWidget "/Game/CANAL/BluePrints/Widgets/BoatColor.BoatColor_C"))
    (Variables|Default|SetInProgress true)
    (bind _output_get (Variables|Default|SetColorUI _returnvalue_2))
    (Variables|/Game/CANAL/BluePrints/Widgets/BoatColor.BoatColor_C|SetTime _output_get _returnvalue)
    (UserInterface|Viewport|AddtoViewport _returnvalue_2 0)
    (Utilities|FlowControl|Delay (Math|Conversions|ToFloat(Integer) (+ _returnvalue 10)))
    (Widget|RemovefromParent _returnvalue_2)
    (Rendering|Material|SetScalarParameterValueonMaterials (Variables|Default|GetLight1) "Light" 0.0)
    (Variables|Default|SetInProgress false)))

(fn ConstructionScript)