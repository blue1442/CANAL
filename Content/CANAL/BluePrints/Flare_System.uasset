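; Interactable flare launcher that fires a flare and then waits for a resupply.
; Interaction, gated by availability and safeguard flags, plays audio and a timeline that moves the flare, then spawns a Flare_Light at the audio component's transform.
; GetNewAmmo resets the flare, shows delivery status on a TextRender through random delays, then animates it back into place and re-arms.
; Each completed resupply lengthens the next wait.
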(event Custom|GetNewAmmo
  (Transformation|SetRelativeLocation (Variables|Default|GetFlare) "0, 0, 0" false false)
  (Rendering|Components|TextRender|SetText (Variables|Default|GetTextRender) (Utilities|Text|ToText(String) "Requesting"))
  (Utilities|FlowControl|Delay (Math|Random|RandomFloatinRange 2e+01 35.0))
  (Rendering|Components|TextRender|SetText (Variables|Default|GetTextRender) (Utilities|Text|ToText(String) "Arriving"))
  (Utilities|FlowControl|Delay (+ (Math|Random|RandomFloatinRange 1e+01 2e+01) (* (Variables|Default|GetFlare_Inc) 7)))
  (bind _newtrack_0 (Timeline|Timeline_0 PlayFromStart)
    (:Update
      (Transformation|SetRelativeLocation (Variables|Default|GetFlare) (Math|Vector|Lerp(Vector) "0, 0, 0" (Variables|Default|GetStarting%20Location) _newtrack_0) false false)
      (Rendering|Components|TextRender|SetText (Variables|Default|GetTextRender) (Utilities|Text|ToText(String) "Arrived"))
      (Variables|Default|SetIsFlare true))
    (:Finished
      (Math|Integer|IncrementInt (Variables|Default|GetFlare_Inc)))))

(event EventBeginPlay
  (bind _asgame_instance (Utilities|Casting|CastToGame_Instance (Game|GetGameInstance)))
  (Variables|Default|SetGame%20Instance _asgame_instance)
  (Variables|Default|SetStarting%20Location (Variables|/Script/Engine.SceneComponent|GetRelativeLocation (Variables|Default|GetFlare)))
  (Rendering|Components|TextRender|SetText (Variables|Default|GetTextRender) (Utilities|Text|ToText(String) "")))

(event EventInteractwithObject
  (if (and (Variables|Default|GetIsFlare) (!= (Variables|Default|GetSafeguard) true))
    (Variables|Default|SetIsFlare false)
    (Variables|Default|SetSafeguard true)
    (Audio|Components|Audio|Play (Variables|Default|GetAudio) 0.0)
    (bind _newtrack_0 (Timeline|Timeline PlayFromStart)
      (:Update
        (Transformation|SetRelativeLocation (Variables|Default|GetFlare) (Math|Vector|Lerp(Vector) (Variables|Default|GetStarting%20Location) "0.000000,0.000000,250.000000" _newtrack_0) false false))
      (:Finished
        (Variables|Default|SetSafeguard false)
        (Game|SpawnActorfromClass "/Game/CANAL/BluePrints/Flare_Light.Flare_Light_C" (Transformation|GetWorldTransform (Variables|Default|GetAudio)) "Undefined" "MultiplyWithRoot" 0 0)
        (CallFunction|GetNewAmmo)))))

(fn ConstructionScript)