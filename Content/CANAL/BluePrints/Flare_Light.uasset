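; Flare light actor that simulates a signal flare rising into the sky, with sound, then burning out.
; On BeginPlay it sets the Flare flag on Game_Instance, and a timeline lerps the point light from a hard-coded world position to ApexHeight while brightening it.
; After a short hold, a second timeline fades the light to zero, then the flag clears and the actor destroys itself.
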(event EventBeginPlay
  (bind _pointlight (Variables|Default|GetPointLight))
  (bind _asgame_instance (Utilities|Casting|CastToGame_Instance (Game|GetGameInstance)))
  (bind _output_get (Variables|Default|SetGame%20Instance _asgame_instance))
  (Variables|/Game/CANAL/BluePrints/Game_Instance.Game_Instance_C|SetFlare _output_get true)
  (Audio|Components|Audio|Play (Variables|Default|GetFlare_sound) 1.0)
  (Rendering|Components|Light|SetIntensity (Variables|Default|GetPointLight) 1e+02)
  (bind _newtrack_0 (Timeline|Timeline PlayFromStart)
    (:Update
      (Transformation|SetWorldLocation _pointlight (Math|Vector|Lerp(Vector) (Math|Vector|MakeVector 581.289378 303.427357 2236.998568) (Variables|Default|GetApex_Height) _newtrack_0) false false)
      (Rendering|Components|Light|SetIntensity _pointlight (Math|Float|Lerp 1.5e+03 3e+03 _newtrack_0)))
    (:Finished
      (Utilities|FlowControl|Delay 4.0)
      (bind _newtrack_0_2 (Timeline|Timeline_0 PlayFromStart)
        (:Update
          (Rendering|Components|Light|SetIntensity _pointlight (Math|Float|Lerp 3e+03 0.0 _newtrack_0_2)))
        (:Finished
          (Variables|/Game/CANAL/BluePrints/Game_Instance.Game_Instance_C|SetFlare (Variables|Default|GetGame%20Instance) false)
          (Actor|DestroyActor))))))

(fn ConstructionScript)