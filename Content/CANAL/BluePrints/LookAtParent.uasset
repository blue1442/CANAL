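; Parent actor, going by its name, for objects that detect whether the player is looking toward them.
; IsObservable compares the negated dot product of the actor-to-pawn direction and the controller's forward vector against LookAtSensitivity.
; It is a view-angle test only, with no trace for occlusion or distance limit.
; Tick runs the check on itself every frame and prints the result when Debug is on.
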(event EventBeginPlay)

(event Collision|EventActorBeginOverlap
  (params (OtherActor :type Actor%20Object%20Reference)))

(event EventTick
  (params (DeltaSeconds :type Float%20%28single-precision%29))
  (bind _isobservable (CallFunction|IsObservable self))
  (if (Variables|Default|GetDebug)
    (if _isobservable
      (Development|PrintString "In View")
      (else
        (Development|PrintString "Not in View")))))

(fn ConstructionScript)

(fn IsObservable
  (params (Actor :type Actor%20Object%20Reference))
  (return (>= (* (Math|Vector|DotProduct (Math|Vector|GetForwardVector (Math|Rotator|FindLookatRotation (Transformation|GetActorLocation Actor) (Transformation|GetActorLocation (Game|Player|GetPlayerPawn 0)))) (Math|Vector|GetForwardVector (Pawn|GetControlRotation (Game|GetPlayerController 0) :!class /Script/Engine.Controller))) -1.0) (Variables|Default|GetLookAtSensitivity))))