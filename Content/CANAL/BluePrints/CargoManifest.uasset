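; Interactable cargo manifest display that blends the player's view to its own camera and shows the boat's cargo on a TextRender.
; Interacting cycles loading text for a randomized number of loops, then, after a matching delay, prints the GameInstance's cargo list if the boat is at sea.
; Tick watches for any key while locked in, showing "Loading Failed" if still loading and blending the view back to the player.
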(event Custom|Lock%20Out%20Prevented
  (bind _player (Variables|Default|GetPlayer))
  (bind _blend_time (Variables|Default|GetBlend%20Time))
  (Development|PrintString "Lock Out Prevented")
  (Game|Player|SetViewTargetwithBlend (Game|GetPlayerController 0) _player _blend_time "VTBlend_Linear" (Variables|Default|GetBlend%20Exp) false)
  (Utilities|FlowControl|Delay _blend_time)
  (Variables|/Game/CANAL/BluePrints/BP_FirstPersonCharacter.BP_FirstPersonCharacter_C|SetInCargoManifest _player false)
  (Variables|Default|SetLock%20in false)
  (Utilities|FlowControl|DoOnce false) ; enters at Reset
)

(event EventBeginPlay
  (bind _loading_counter (Variables|Default|GetLoading%20Counter))
  (bind _asgame_instance (Utilities|Casting|CastToGame_Instance (Game|GetGameInstance)))
  (Variables|Default|SetGame%20Instance _asgame_instance)
  (bind _asbp_first_person_character (Utilities|Casting|CastToBP_FirstPersonCharacter (Game|GetPlayerCharacter 0)))
  (Variables|Default|SetPlayer _asbp_first_person_character)
  (Utilities|Array|SetArrayElem _loading_counter 2 (Math|Random|RandomIntegerinRange (Utilities|Array|Get(acopy) _loading_counter) (Utilities|Array|Get(acopy) _loading_counter 1))))

(event EventInteractwithObject
  (bind _returnvalue (Game|GetPlayerCharacter 0))
  (bind _game_instance (Variables|Default|GetGame%20Instance))
  (bind _springarm (Variables|Default|GetSpringArm))
  (bind _returnvalue_2 (Transformation|GetActorLocation _returnvalue))
  (bind _returnvalue_3 (Transformation|GetWorldLocation _springarm))
  (Variables|Default|SetInc 0)
  (Variables|Default|SetLoadingStatus false)
  (Utilities|FlowControl|Sequence
    (:then_0
      ;[1 1 1] When Entering StartCamera
      (Variables|/Game/CANAL/BluePrints/BP_FirstPersonCharacter.BP_FirstPersonCharacter_C|SetInCargoManifest (Variables|Default|GetPlayer) true)
      (Game|Player|SetViewTargetwithBlend (Game|GetPlayerController 0) self (Variables|Default|GetBlend%20Time) "VTBlend_Cubic" (Variables|Default|GetBlend%20Exp) false)
      (Utilities|FlowControl|Delay (Variables|Default|GetBlend%20Time))
      (Variables|Default|SetLock%20in true)
      ;;[1 1 1] Set the offset only one
      (Utilities|FlowControl|DoOnce false
        (:Completed
          (Development|PrintString (Utilities|String|ToString(Vector) _returnvalue_3))
          (Development|PrintString (Utilities|String|ToString(Vector) _returnvalue_2))
          (Variables|Default|SetOffset (- _returnvalue_3 _returnvalue_2)))))
    (:then_1
      ;[1 1 1] Loading Text
      (Variables|Default|SetLoadingStatus true)
      (bind _index (Utilities|ForLoopwithDelay 0 2 (Variables|Default|GetDuration) :!label _label)
        (:Loop%20Body
          (Development|PrintString (Utilities|Array|Get(acopy) (Variables|Default|GetLoading) _index))
          (if (Variables|Default|GetLoadingStatus)
            (Rendering|Components|TextRender|SetText (Variables|Default|GetTextRender) (Utilities|Text|ToText(String) (Utilities|Array|Get(acopy) (Variables|Default|GetLoading) _index)))
            (else
              (goto _label Break))))
        (:Completed
          (bind _result (Math|Integer|IncrementInt (Variables|Default|GetInc))
            (:%20%20
              (if (Variables|Default|GetLoadingStatus)
                (if (== _result (Utilities|Array|Get(acopy) (Variables|Default|GetLoading%20Counter) 2))
                  (Development|PrintString "Loading Completing")
                  (else
                    (goto _label)))
                (else
                  (goto _label Break))))))))
    (:then_2
      ;[1 1 1] Show the Manifest
      (if (Variables|Default|GetLoadingStatus)
        (Utilities|FlowControl|Delay (* (* (Utilities|Array|Get(acopy) (Variables|Default|GetLoading%20Counter) 2) 3) (Variables|Default|GetDuration)))
        (Variables|Default|SetList "")
        (if (Variables|/Game/CANAL/BluePrints/Game_Instance.Game_Instance_C|GetBoatOnSea _game_instance)
          (for _array_element (Variables|/Game/CANAL/BluePrints/Game_Instance.Game_Instance_C|GetBoatCargo _game_instance)
            (Variables|Default|SetList (Utilities|String|Append (Variables|Default|GetList) _array_element " 
")))
          (if (Variables|Default|GetLoadingStatus)
            (Rendering|Components|TextRender|SetText (Variables|Default|GetTextRender) (Utilities|Text|ToText(String) (Variables|Default|GetList)))
            (Variables|Default|SetLoadingStatus false)))))))

(event EventTick
  (params (DeltaSeconds :type Float%20%28single-precision%29))
  (if (and (Game|Player|IsInputKeyDown (Game|GetPlayerController 0) "AnyKey") (Variables|Default|GetLock%20in))
    (if (Variables|Default|GetLoadingStatus)
      (Variables|Default|SetLoadingStatus false)
      (Rendering|Components|TextRender|SetText (Variables|Default|GetTextRender) (Utilities|Text|ToText(String) "Loading Failed")))
    (Utilities|FlowControl|DoOnce false
      (:Completed
        (CallFunction|LockOutPrevented)))))

(fn ConstructionScript)