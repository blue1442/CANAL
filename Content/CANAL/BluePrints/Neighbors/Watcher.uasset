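; Watcher is an actor that constantly turns to face the player pawn and creeps toward it.
; Each Tick measures the distance and sets a look-at rotation, adding small random jitter on every axis when the player is within range.
; It then moves along the look-at direction without sweep, with a step divided by delta time, so its speed depends on frame rate.
; BeginPlay prints the starting distance, and a direction debug print is left unconnected.
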(event EventTick
  (params (DeltaSeconds :type Float%20%28single-precision%29))
  (bind _returnvalue (Transformation|GetActorLocation))
  (bind _returnvalue_2 (Game|Player|GetPlayerPawn 0))
  (bind _returnvalue_3 (Transformation|GetActorLocation _returnvalue_2))
  (bind _returnvalue_4 (Math|Rotator|FindLookatRotation _returnvalue _returnvalue_3))
  (bind (_roll _pitch _yaw) (Math|Rotator|BreakRotator _returnvalue_4))
  (bind _output_get (Variables|Default|SetDistance (Math|Vector|Distance(Vector) (Transformation|GetActorLocation) (Transformation|GetActorLocation (Game|Player|GetPlayerPawn 0)))))
  (if (<= _output_get 2.5e+04)
    (Variables|Default|SetPointRotation (Math|Rotator|MakeRotator (+ _roll (Math|Random|RandomFloatinRange -1.0 1.0)) (+ (Math|Random|RandomFloatinRange -1.0 1.0) _pitch) (+ _yaw (Math|Random|RandomFloatinRange -1.0 1.0))))
    (else
      (Variables|Default|SetPointRotation _returnvalue_4)))
  (Transformation|SetActorRotation (Variables|Default|GetPointRotation))
  (Transformation|SetActorLocation (+ (/ (Math|Vector|GetForwardVector _returnvalue_4) (/ DeltaSeconds 0.1)) (Transformation|GetActorLocation)) false false))

(event EventBeginPlay
  (bind _output_get (Variables|Default|SetDistance (Math|Vector|Distance(Vector) (Transformation|GetActorLocation) (Transformation|GetActorLocation (Game|Player|GetPlayerPawn 0)))))
  (Development|PrintString (Utilities|String|ToString(Float) _output_get)))

(fn ConstructionScript)