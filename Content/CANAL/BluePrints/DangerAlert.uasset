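; DangerAlert is a four-stage warning light that shows the danger level based on the number wrong stored in the Game Instance.
; On BeginPlay it caches the Game Instance and runs SetDangerLevel, which maps NumWrong from zero to three onto green, yellow, orange and red.
; Each matched level first zeroes the "Light" scalar material parameter on all four components, then sets it to LightValue on the active one.
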(event Custom|Set%20Danger%20Level
  (bind _light_value (Variables|Default|GetLight%20Value))
  (switch int (Variables|/Game/CANAL/BluePrints/Game_Instance.Game_Instance_C|GetNumWrong (Variables|Default|GetGame%20Instance))
    (:0
      (CallFunction|TurnOffLights)
      (Rendering|Material|SetScalarParameterValueonMaterials (Variables|Default|GetDangerGreen) "Light" _light_value))
    (:1
      (CallFunction|TurnOffLights)
      (Rendering|Material|SetScalarParameterValueonMaterials (Variables|Default|GetDangerYellow) "Light" _light_value))
    (:2
      (CallFunction|TurnOffLights)
      (Rendering|Material|SetScalarParameterValueonMaterials (Variables|Default|GetDangerOrange) "Light" _light_value))
    (:3
      (CallFunction|TurnOffLights)
      (Rendering|Material|SetScalarParameterValueonMaterials (Variables|Default|GetDangerRed) "Light" _light_value))))

(event EventBeginPlay
  (bind _asgame_instance (Utilities|Casting|CastToGame_Instance (Game|GetGameInstance)))
  (Variables|Default|SetGame%20Instance _asgame_instance)
  (CallFunction|SetDangerLevel))

(fn ConstructionScript)

(fn TurnOffLights
  (Rendering|Material|SetScalarParameterValueonMaterials (Variables|Default|GetDangerGreen) "Light" 0.0)
  (return))