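; Canal buoy actor that lights its two middle meshes and animates a floating motion from BeginPlay.
; It sets the "Light" material parameter on both meshes, then starts separate roll and vertical timelines.
; Each timeline alternates forward and reverse through a FlipFlop on Finished for continuous ping-pong motion.
; The vertical timeline writes relative Z directly from the scaled track, replacing the placed height rather than offsetting it.
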(event Custom|Bobbing
  (bind _returnvalue (Transformation|GetActorRotation))
  (bind (_roll _pitch _yaw) (Math|Rotator|BreakRotator _returnvalue))
  (bind _track1 (Timeline|Timeline Play)
    (:Update
      (Transformation|SetActorRotation (Math|Rotator|MakeRotator _track1 _pitch _yaw)))
    (:Finished
      (Utilities|FlowControl|FlipFlop
        (:A
          (Timeline|Timeline ReverseFromEnd))
        (:B
          (Timeline|Timeline PlayFromStart))))))

(event Custom|UpnDown
  (bind _returnvalue (Transformation|GetActorLocation))
  (bind (_x _y) (Math|Vector|BreakVector _returnvalue))
  (bind _newtrack_0 (Timeline|Timeline_0 Play)
    (:Update
      (Transformation|SetActorRelativeLocation (Math|Vector|MakeVector _x _y (* _newtrack_0 25.0))))
    (:Finished
      (Utilities|FlowControl|FlipFlop
        (:A
          (Timeline|Timeline_0 ReverseFromEnd))
        (:B
          (Timeline|Timeline_0 PlayFromStart))))))

(event EventBeginPlay
  (Utilities|FlowControl|Sequence
    (:then_0
      (Rendering|Material|SetScalarParameterValueonMaterials (Variables|Default|GetMiddleLight_1) "Light" 1.0))
    (:then_1
      (CallFunction|Bobbing))
    (:then_2
      (CallFunction|UpnDown))))

(fn ConstructionScript)