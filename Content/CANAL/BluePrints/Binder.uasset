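; Interactable binder that the player opens and closes to read rules on screen.
; Each interaction plays a page-turn sound and alternates via a FlipFlop between opening and closing.
; Opening snaps the spine and top to open transforms and adds a Pages widget to the viewport, while closing resets both parts and removes it.
; The first-person character's InAction flag is set while the binder is open and cleared on close.
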(event EventInteractwithObject
  (bind _spine (Variables|Default|GetSpine))
  (Variables|Default|SetPlayer (Game|GetPlayerCharacter 0))
  (Development|PrintString "Opening Rules")
  (Audio|PlaySound2D "/Game/CANAL/Sounds/PageTurn.PageTurn" 1.0 1.0 0.0 0 0)
  (Utilities|FlowControl|FlipFlop
    (:A
      (Transformation|SetRelativeLocationAndRotation _spine "17.000000,28.000000,0.000000" "0.000000,90.000000,0.000000" false false)
      (Transformation|SetRelativeLocationAndRotation (Variables|Default|GetTop) "0.000000,55.000000,0.000000" "0.000000,180.000000,0.000000" false false)
      (Variables|Default|SetOpen true)
      (bind _returnvalue (UserInterface|CreateWidget "/Game/CANAL/BluePrints/Widgets/Pages.Pages_C"))
      (bind _output_get (Variables|Default|SetPages _returnvalue))
      (UserInterface|Viewport|AddtoViewport _output_get 0)
      (bind _asbp_first_person_character (Utilities|Casting|CastToBP_FirstPersonCharacter (Variables|Default|GetPlayer)))
      (Variables|/Game/CANAL/BluePrints/BP_FirstPersonCharacter.BP_FirstPersonCharacter_C|SetInAction _asbp_first_person_character true))
    (:B
      (Transformation|SetRelativeLocationAndRotation _spine "0, 0, 0" "0, 0, 0" false false)
      (Variables|Default|SetOpen false)
      (Widget|RemovefromParent (Variables|Default|GetPages))
      (bind _asbp_first_person_character_2 (Utilities|Casting|CastToBP_FirstPersonCharacter (Variables|Default|GetPlayer)))
      (Variables|/Game/CANAL/BluePrints/BP_FirstPersonCharacter.BP_FirstPersonCharacter_C|SetInAction _asbp_first_person_character_2 false))))

(fn ConstructionScript
  (|CallParentFunction))