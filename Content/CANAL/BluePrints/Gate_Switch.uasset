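; Lever switch actor that operates a linked Gate when interacted with.
; If the Gate's Safeguard flag is true and the lever is idle, it triggers the Gate, plays a sound and alternates full up/down throws through a FlipFlop.
; If Safeguard is false, a short timeline only nudges the lever from its current end, tracked by UpOrDown.
; Timelines lerp the lever's transform, with IsInUse blocking input during full throws.
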(event EventBeginPlay
  (Transformation|SetRelativeLocationAndRotation (Variables|Default|GetLever) "54.000000,0.000000,-12.000000" "0, 0, 0" false false)
  (Variables|Default|SetUp%20or%20Down true))

(event Collision|EventActorBeginOverlap
  (params (OtherActor :type Actor%20Object%20Reference)))

(event EventTick
  (params (DeltaSeconds :type Float%20%28single-precision%29)))

(event EventInteractwithObject
  (bind _gate (Variables|Default|GetGate))
  (bind _lever (Variables|Default|GetLever))
  (bind _lever_2 (Variables|Default|GetLever))
  (if (Variables|/Game/CANAL/BluePrints/Gate.Gate_C|GetSafeguard _gate)
    (if (not (Variables|Default|GetIs%20in%20use))
      (Default|InteractwithObject _gate)
      (Audio|PlaySound2D "/Game/CANAL/Sounds/lever_sound.lever_sound" 1.0 1.0 0.0 0 0)
      (Utilities|FlowControl|FlipFlop
        (:A
          (Variables|Default|SetIs%20in%20use true)
          (bind _newtrack_0 (Timeline|Timeline PlayFromStart)
            (:Update
              (Transformation|SetRelativeLocationAndRotation _lever (Math|Vector|Lerp(Vector) "54.000000,0.000000,-12.000000" "54.000000,15.000000,4.000000" _newtrack_0) (Math|Rotator|Lerp(Rotator) "0.000000,0.000000,0.000000" "0.000000,0.000000,-90.000000" _newtrack_0) false false))
            (:Finished
              (Variables|Default|SetIs%20in%20use false)
              (Variables|Default|SetUp%20or%20Down false))))
        (:B
          (Variables|Default|SetIs%20in%20use true)
          (bind _newtrack_0_2 (Timeline|Lerp PlayFromStart)
            (:Update
              (Transformation|SetRelativeLocationAndRotation _lever (Math|Vector|Lerp(Vector) "54.000000,15.000000,4.000000" "54.000000,0.000000,-12.000000" _newtrack_0_2) (Math|Rotator|Lerp(Rotator) "0.000000,0.000000,-90.000000" "0.000000,0.000000,-0.000000" _newtrack_0_2) false false))
            (:Finished
              (Variables|Default|SetIs%20in%20use false)
              (Variables|Default|SetUp%20or%20Down true))))))
    (elif (Variables|Default|GetUp%20or%20Down)
      (bind _newtrack_0_3 (Timeline|Timeline_0 PlayFromStart)
        (:Update
          (Transformation|SetRelativeLocationAndRotation _lever_2 (Math|Vector|Lerp(Vector) "54.000000,0.000000,-12.000000" "54.000000,2.316912,-13.622319" _newtrack_0_3) (Math|Rotator|Lerp(Rotator) "0.000000,0.000000,0.000000" "0.000000,0.000000,-10.000000" _newtrack_0_3) false false)))
      (else
        (bind _newtrack_0_4 (Timeline|Timeline_1 PlayFromStart)
          (:Update
            (Transformation|SetRelativeLocationAndRotation _lever_2 (Math|Vector|Lerp(Vector) "54.000000,15.000000,4.000000" "54.000000,14.607127,-1.509440" _newtrack_0_4) (Math|Rotator|Lerp(Rotator) "0.000000,0.000000,-90.000000" "0.000000,0.000000,-80.000000" _newtrack_0_4) false false)))))))

(fn ConstructionScript
  (|CallParentFunction))