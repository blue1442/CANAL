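; An interactable double gate that toggles between open and closed.
; InteractwithObject alternately plays and reverses a Timeline that rotates the left and right gates 90 degrees in opposite directions.
; A Safeguard flag ignores further interaction while the gates move.
; When the Timeline finishes, a second FlipFlop updates GateStatus and GateClosed on the Game Instance and prints the new state.
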(event EventBeginPlay
  (bind _asgame_instance (Utilities|Casting|CastToGame_Instance (Game|GetGameInstance)))
  (Variables|Default|SetGame%20Instance _asgame_instance))

(event EventInteractwithObject
  (bind _game_instance (Variables|Default|GetGame%20Instance))
  (if (Variables|Default|GetSafeguard)
    (Utilities|FlowControl|FlipFlop
      (:A
        (bind _alpha1 (Timeline|Timeline Play)
          (:Update
            (Variables|Default|SetSafeguard false)
            (Transformation|SetRelativeRotation (Variables|Default|GetRightGate) (Math|Rotator|Lerp(Rotator) "0, 0, 0" "0,90.000000, 0" _alpha1) false false)
            (Transformation|SetRelativeRotation (Variables|Default|GetLeftGate) (Math|Rotator|Lerp(Rotator) "0, 0, 0" "0,-90.000000, 0" _alpha1) false false))
          (:Finished
            (Variables|Default|SetSafeguard true)
            (Utilities|FlowControl|FlipFlop
              (:A
                (Variables|Default|SetGate_Status false)
                (Development|PrintString "gate is Open")
                (Variables|/Game/CANAL/BluePrints/Game_Instance.Game_Instance_C|SetGate_Closed _game_instance false))
              (:B
                (Variables|Default|SetGate_Status true)
                (Development|PrintString "gate is Closed")
                (Variables|/Game/CANAL/BluePrints/Game_Instance.Game_Instance_C|SetGate_Closed _game_instance true))))))
      (:B
        (Timeline|Timeline ReverseFromEnd)))))

(fn ConstructionScript
  (|CallParentFunction))