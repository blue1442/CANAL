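; BoatApproachingAlert is an actor that lights a warning lamp while a boat is on the sea.
; On BeginPlay it caches the game instance, then runs a self-repeating check every two seconds.
; Each check reads the BoatOnSea flag and switches the "Light" material scalar on its Sphere and StaticMesh components between glowing and off.
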(event Custom|CheckLight
  (bind _sphere (Variables|Default|GetSphere))
  (if (Variables|/Game/CANAL/BluePrints/Game_Instance.Game_Instance_C|GetBoatOnSea (Variables|Default|GetGame%20Instance))
    (Rendering|Material|SetScalarParameterValueonMaterials _sphere "Light" 25.0)
    (else
      (Rendering|Material|SetScalarParameterValueonMaterials _sphere "Light" 0.0)))
  (Utilities|FlowControl|Delay 2.0)
  (CallFunction|CheckLight))

(event EventBeginPlay
  (bind _asgame_instance (Utilities|Casting|CastToGame_Instance (Game|GetGameInstance)))
  (Variables|Default|SetGame%20Instance _asgame_instance)
  (CallFunction|CheckLight))

(fn ConstructionScript)