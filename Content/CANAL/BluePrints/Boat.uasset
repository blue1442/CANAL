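; Boat actor for a canal-crossing game that spawns with a random code, lights, color and cargo, then checks whether it may cross.
; Validation tests code, lights and cargo rules and sets a validity flag, while code, color and cargo are copied to the Game Instance.
; Timelines drive it along an approach spline, then onto the canal or leaving spline depending on GateClosed.
; Other timelines handle hull sway and animate light brightness.
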(event Custom|Move%20Object
  (bind _spline_boat_ref (Variables|Default|GetSpline%20Boat%20Ref))
  (bind _spline (Variables|/Game/CANAL/BluePrints/BoatPath.BoatPath_C|GetSpline _spline_boat_ref))
  (Components|Timeline|SetPlayRate (Variables|Default|GetMove%20Object%20T) (/ 1.0 (Variables|Default|GetTime%20to%20Complete)))
  (bind _newtrack_0 (Timeline|Move%20Object%20T Play)
    (:Update
      (Transformation|SetActorTransform (Math|Transform|MakeTransform (Spline|GetLocationatDistanceAlongSpline _spline (Math|Float|Lerp 0.0 (Spline|GetSplineLength (Variables|/Game/CANAL/BluePrints/BoatPath.BoatPath_C|GetSpline (Variables|Default|GetSpline%20Boat%20Ref))) _newtrack_0) "World") (Spline|GetRotationatDistanceAlongSpline _spline (Math|Float|Lerp 0.0 (Spline|GetSplineLength (Variables|/Game/CANAL/BluePrints/BoatPath.BoatPath_C|GetSpline (Variables|Default|GetSpline%20Boat%20Ref))) _newtrack_0) "World"))))
    (:Finished
      (CallFunction|CanalorLeave))))

(event Custom|Canal%20or%20Leave
  (bind _spline_boat_leaving (Variables|Default|GetSpline%20Boat%20Leaving))
  (bind _spline_boat_canal (Variables|Default|GetSpline%20Boat%20Canal))
  (bind _spline (Variables|/Game/CANAL/BluePrints/BoatPath_Leaving.BoatPath_Leaving_C|GetSpline _spline_boat_leaving))
  (bind _spline_2 (Variables|/Game/CANAL/BluePrints/BoatPath_Canal.BoatPath_Canal_C|GetSpline _spline_boat_canal))
  (if (Variables|/Game/CANAL/BluePrints/Game_Instance.Game_Instance_C|GetGate_Closed (Variables|Default|GetGame%20Instance))
    (Development|PrintString "gate is closed, leaving canal")
    (Components|Timeline|SetPlayRate (Variables|Default|GetMove%20Object%20T2) (/ 1.0 (Variables|Default|GetTime%20to%20Complete)))
    (bind _newtrack_0 (Timeline|Move%20Object%20T2 Play)
      (:Update
        (Transformation|SetActorTransform (Math|Transform|MakeTransform (Spline|GetLocationatDistanceAlongSpline _spline (Math|Float|Lerp 0.0 (Spline|GetSplineLength (Variables|/Game/CANAL/BluePrints/BoatPath_Leaving.BoatPath_Leaving_C|GetSpline (Variables|Default|GetSpline%20Boat%20Leaving))) _newtrack_0) "World") (Spline|GetRotationatDistanceAlongSpline _spline (Math|Float|Lerp 0.0 (Spline|GetSplineLength (Variables|/Game/CANAL/BluePrints/BoatPath_Leaving.BoatPath_Leaving_C|GetSpline (Variables|Default|GetSpline%20Boat%20Leaving))) _newtrack_0) "World")))))
    (else
      (Development|PrintString "gate is open, entering canal")
      (Components|Timeline|SetPlayRate (Variables|Default|GetMove%20Object%20T3) (/ 1.0 (Variables|Default|GetTime%20to%20Complete)))
      (bind _newtrack_0_2 (Timeline|Move%20Object%20T3 Play)
        (:Update
          (Transformation|SetActorTransform (Math|Transform|MakeTransform (Spline|GetLocationatDistanceAlongSpline _spline_2 (Math|Float|Lerp 0.0 (Spline|GetSplineLength (Variables|/Game/CANAL/BluePrints/BoatPath_Canal.BoatPath_Canal_C|GetSpline (Variables|Default|GetSpline%20Boat%20Canal))) _newtrack_0_2) "World") (Spline|GetRotationatDistanceAlongSpline _spline_2 (Math|Float|Lerp 0.0 (Spline|GetSplineLength (Variables|/Game/CANAL/BluePrints/BoatPath_Canal.BoatPath_Canal_C|GetSpline (Variables|Default|GetSpline%20Boat%20Canal))) _newtrack_0_2) "World"))))))))

(event Custom|Randomize%20Boat
  (Utilities|FlowControl|Sequence
    (:then_0
      (switch int (Math|Integer|%(Integer) (Math|Random|RandomInteger 100) 7)
        (:Default
          (Variables|CodeStructure|SetStartingCodeIndex 0 :!label _label))
        (:0
          (Variables|CodeStructure|SetStartingCodeIndex 2))
        (:1
          (Variables|CodeStructure|SetStartingCodeIndex 1 :!label _label_2))
        (:2
          (goto _label_2))
        (:3
          (goto _label))
        (:4
          (goto _label))
        (:5
          (goto _label))
        (:6
          (goto _label)))
      (Variables|Identifer|SetCode (Utilities|String|Append (Variables|Identifer|GetCode) (Utilities|Array|Get(acopy) (Variables|CodeStructure|GetCodeStart) (Variables|CodeStructure|GetStartingCodeIndex))))
      (for _index (range 0 1)
        (Variables|Identifer|SetCode (Utilities|String|Append (Variables|Identifer|GetCode) (Utilities|Array|Get(acopy) (Variables|CodeStructure|GetAlphabet) (Math|Random|RandomInteger 14)))))
      (bind _output_get (Variables|Identifer|SetCode (Utilities|String|Append (Variables|Identifer|GetCode) "-" (Utilities|String|ToString(Integer) (Math|Random|RandomInteger 10)))))
      (Development|PrintString _output_get))
    (:then_1
      (bind _output_get_2 (Variables|LightStructure|SetLightInt (Math|Random|RandomIntegerinRange 1 3)))
      (bind _output_get_3 (Variables|Identifer|SetLights (.Value (Utilities|Map|Find (Variables|LightStructure|GetLightMap) _output_get_2))))
      (Development|PrintString _output_get_3)
      (Rendering|Material|SetMaterial (Variables|Default|GetLight6) 0 (.Value (Utilities|Map|Find (Variables|Default|GetLight%20Material) _output_get_2)))
      (Rendering|Material|SetScalarParameterValueonMaterials (Variables|Default|GetLight1) "Light" 15.0))
    (:then_2
      (bind _output_get_4 (Variables|Identifer|SetColor (.Value (Utilities|Map|Find (Variables|ColorStructure|GetColorMap) (Math|Random|RandomIntegerinRange 1 3)))))
      (Development|PrintString _output_get_4))
    (:then_3
      (for _index_2 (range 0 (Math|Random|RandomIntegerinRange 1 3))
        (Utilities|Array|Add (Variables|CargoStructure|GetCargoList) (.Value (Utilities|Map|Find (Variables|CargoStructure|GetCargo%20Map) (Math|Random|RandomIntegerinRange 1 3)))))
      (for _array_element (Variables|CargoStructure|GetCargoList)
        (Development|PrintString _array_element)))))

(event Custom|Is_Boat_Valid?
  (bind _code (Variables|Identifer|GetCode))
  (bind _boat_validation (Variables|Default|GetBoat_Validation))
  ;[1 1 1] Boat checks itself and sees if its a valid boat to cross the canal
  (Utilities|FlowControl|Sequence
    (:then_0
      (switch string (Utilities|String|GetSubstring (Variables|Identifer|GetCode) 0)
        (:X
          (if (>= (Math|Conversions|ToInteger(Byte) (Utilities|String|GetSubstring (Variables|Identifer|GetCode) 4)) 3)
            (Utilities|Array|SetArrayElem _boat_validation 0 true)
            (else
              (Utilities|Array|SetArrayElem _boat_validation 0 false))))
        (:A
          (bind _array_element (Utilities|Array|ForEachLoopwithBreak (Variables|Default|GetVowels) :!label _label)
            (:LoopBody
              (if (and (== (Math|Integer|%(Integer) (Math|Conversions|ToInteger(Byte) (Utilities|String|GetSubstring _code 4)) 2) 0) (Utilities|String|Contains _code _array_element))
                (Utilities|Array|SetArrayElem (Variables|Default|GetBoat_Validation) 0 true)
                (goto _label Break)))))
        (:F
          (if (Utilities|Enum|Equal(Enum) (Variables|Identifer|GetLights) "Blue")
            (Utilities|Array|SetArrayElem (Variables|Default|GetBoat_Validation) 0 true)))))
    (:then_1
      (switch string (Variables|Identifer|GetLights)
        (:White
          (Utilities|Array|SetArrayElem (Variables|Default|GetBoat_Validation) 1 true))
        (:Yellow
          (switch string (Variables|Identifer|GetColor)
            (:White
              _)
            (:Red
              _))
          (Utilities|Array|SetArrayElem (Variables|Default|GetBoat_Validation) 1 true))))
    (:then_2
      (if (not (Utilities|Array|ContainsItem (Variables|CargoStructure|GetCargoList) "Weapons"))
        (Utilities|Array|SetArrayElem (Variables|Default|GetBoat_Validation) 2 true)))
    (:then_3
      (for _array_element_2 (Variables|Default|GetBoat_Validation)
        (if (== _array_element_2 true)
          (Math|Integer|IncrementInt (Variables|Default|GetValidation%20Count))))
      (if (>= (Variables|Default|GetValidation%20Count) 3)
        (Variables|Default|SetIs_Boat_Valid true)
        (Development|PrintString "Boat is Valid!" true true "(R=0.000000,G=1.000000,B=0.101851,A=1.000000)")
        (else
          (Development|PrintString "Boat is not valid!" true true "(R=1.000000,G=0.046830,B=0.000000,A=1.000000)"))))))

(event Custom|Sway
  (bind _defaultsceneroot (Variables|Default|GetDefaultSceneRoot))
  (bind _relativerotation (Variables|/Script/Engine.SceneComponent|GetRelativeRotation _defaultsceneroot))
  (bind (_roll _pitch _yaw) (Math|Rotator|BreakRotator _relativerotation))
  (bind _track (Timeline|Bobbing Play)
    (:Update
      (Transformation|SetRelativeRotation _defaultsceneroot (Math|Rotator|MakeRotator (* _track 5.0) _pitch _yaw) false false))
    (:Finished
      (Utilities|FlowControl|FlipFlop
        (:A
          (Timeline|Bobbing ReverseFromEnd))
        (:B
          (Timeline|Bobbing PlayFromStart))))))

(event Custom|BoatLights
  (bind _newtrack_0 (Timeline|Timeline Play)
    (:Update
      (Rendering|Material|SetScalarParameterValueonMaterials (Variables|Default|GetLight1) "Light" (* _newtrack_0 15.0)))))

(event EventBeginPlay
  (Utilities|FlowControl|Sequence
    (:then_0
      (bind _returnvalue (Actor|GetActorOfClass "/Game/CANAL/BluePrints/BoatPath.BoatPath_C"))
      (Variables|Default|SetSpline%20Boat%20Ref _returnvalue)
      (CallFunction|MoveObject))
    (:then_1
      (bind _returnvalue_2 (Actor|GetActorOfClass "/Game/CANAL/BluePrints/BoatPath_Canal.BoatPath_Canal_C"))
      (Variables|Default|SetSpline%20Boat%20Canal _returnvalue_2))
    (:then_2
      (bind _returnvalue_3 (Actor|GetActorOfClass "/Game/CANAL/BluePrints/BoatPath_Leaving.BoatPath_Leaving_C"))
      (Variables|Default|SetSpline%20Boat%20Leaving _returnvalue_3))
    (:then_3
      (bind _asgame_instance (Utilities|Casting|CastToGame_Instance (Game|GetGameInstance)))
      (bind _output_get (Variables|Default|SetGame%20Instance _asgame_instance))
      (Variables|/Game/CANAL/BluePrints/Game_Instance.Game_Instance_C|SetBoatOnSea _output_get true))
    (:then_4
      (CallFunction|RandomizeBoat)
      (CallFunction|IsBoatValid?)
      (Variables|/Game/CANAL/BluePrints/Game_Instance.Game_Instance_C|SetCurrent_Boat_Name (Variables|Default|GetGame%20Instance) (Variables|Identifer|GetCode))
      (Variables|/Game/CANAL/BluePrints/Game_Instance.Game_Instance_C|SetBoatColor (Variables|Default|GetGame%20Instance) (Variables|Identifer|GetColor))
      (Variables|/Game/CANAL/BluePrints/Game_Instance.Game_Instance_C|SetBoatCargo (Variables|Default|GetGame%20Instance) (Variables|CargoStructure|GetCargoList)))
    (:then_5
      (CallFunction|Sway)
      (CallFunction|BoatLights))))

(fn ConstructionScript)