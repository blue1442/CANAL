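; BoatPapers is an actor that displays the current boat's papers: VIN code, origin and stamp, with an animated pulldown screen.
; BeginPlay caches the Game Instance and the starting stamp and screen transforms, and hides the stamp.
; GetBoatDetails fills the text and stamp material (via map lookup) from BoatStructInfo, then plays a load sound.
; It randomly jitters the stamp's position and pitch, and a Timeline lerps the screen from its reset transform.
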(event Custom|GetBoatDetails
  (bind _game_instance (Variables|Default|GetGame%20Instance))
  (bind _stamptransform (Variables|Default|GetStampTransform))
  (bind _stamp (Variables|Default|GetStamp))
  (bind (_location _rotation _scale) (Math|Transform|BreakTransform _stamptransform))
  (bind _boatstructinfo (Variables|/Game/CANAL/BluePrints/Game_Instance.Game_Instance_C|GetBoatStructInfo _game_instance))
  (bind (_code _lights _cargo _color _vin_code _origin _stamp_2) (Utilities|Struct|BreakBoatInfoStruct _boatstructinfo))
  (bind (_roll _pitch _yaw) (Math|Rotator|BreakRotator _rotation))
  (bind (_x _y _z) (Math|Vector|BreakVector _location))
  (Transformation|SetRelativeTransform (Variables|Default|GetPulldownScreen) (Variables|Default|GetPulldownScreenTransform) false false)
  (Rendering|Components|TextRender|SetText (Variables|Default|GetTop) (Utilities|Text|ToText(String) _vin_code))
  (Rendering|Components|TextRender|SetText (Variables|Default|GetOrigin) (Utilities|Text|ToText(String) _origin))
  (Rendering|Material|SetMaterial _stamp 0 (.Value (Utilities|Map|Find (Variables|Default|GetStampMatMap) _stamp_2)))
  (Rendering|SetVisibility _stamp true false)
  (Audio|PlaySoundatLocation "/Game/CANAL/Sounds/ScreenLoad.ScreenLoad" (Transformation|GetActorLocation) "0, 0, 0" 0.3 1.0 0.0 "/Game/CANAL/Sounds/Attenuation/CloseRange.CloseRange" 0 0 0)
  (Transformation|SetRelativeTransform (Variables|Default|GetStamp) (Math|Transform|MakeTransform (Math|Vector|MakeVector (+ _x (Math|Random|RandomFloatinRange -5.0 5.0)) _y (+ _z (Math|Random|RandomFloatinRange -5.0 5.0))) (Math|Rotator|MakeRotator _roll (+ _pitch (Math|Random|RandomFloatinRange -25.0 25.0)) _yaw) _scale) false false)
  (bind _newtrack_0 (Timeline|Timeline PlayFromStart)
    (:Update
      (Transformation|SetRelativeTransform (Variables|Default|GetPulldownScreen) (Math|Transform|Lerp(Transform) (Variables|Default|GetPulldownScreenTransform) (Math|Transform|MakeTransform "0.000000,50.822610,-44.203186" "0.000000,0.000000,90.000000" "0.908783,0.003336,1.542337") _newtrack_0) false false))))

(event EventBeginPlay
  (bind _asgame_instance (Utilities|Casting|CastToGame_Instance (Game|GetGameInstance)))
  (Variables|Default|SetGame%20Instance _asgame_instance)
  (Rendering|SetVisibility (Variables|Default|GetStamp) false false)
  (Variables|Default|SetStampTransform (Transformation|GetRelativeTransform (Variables|Default|GetStamp)))
  (Variables|Default|SetPulldownScreenTransform (Transformation|GetRelativeTransform (Variables|Default|GetPulldownScreen))))

(event Collision|EventActorBeginOverlap
  (params (OtherActor :type Actor%20Object%20Reference)))

(event EventTick
  (params (DeltaSeconds :type Float%20%28single-precision%29)))

(fn ConstructionScript)