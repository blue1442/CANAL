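; Interactable monitor that spells out the current boat's name one letter at a time on its TextRender.
; On interaction it reads CurrentBoatName from the Game_Instance cached at BeginPlay, then steps through it with a delayed loop, replacing the displayed character about every second.
; A SafeGuard flag blocks retriggering until the loop completes, and debug prints trace each step.
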(event Custom|PlayOneLetterAAT
  (bind _index (Utilities|ForLoopwithDelay 0 (Utilities|String|Len (Variables|Default|GetBoatName)) 1.0)
    (:Loop%20Body
      (Development|PrintString (Utilities|String|ToString(Integer) _index))
      (Development|PrintString (Utilities|String|GetSubstring (Variables|Default|GetBoatName) _index))
      (Rendering|Components|TextRender|SetText (Variables|Default|GetTextRender) (Utilities|Text|ToText(String) (Utilities|String|GetSubstring (Variables|Default|GetBoatName) _index))))
    (:Completed
      (Variables|Default|SetSafeGuard true)
      (Development|PrintString "Name is Done"))))

(event EventBeginPlay
  (bind _asgame_instance (Utilities|Casting|CastToGame_Instance (Game|GetGameInstance)))
  (Variables|Default|SetGame%20Instance _asgame_instance))

(event EventInteractwithObject
  (Development|PrintString "Text Button Pressed")
  (if (Variables|Default|GetSafeGuard)
    (Variables|Default|SetSafeGuard false)
    (bind _output_get (Variables|Default|SetBoatName (Variables|/Game/CANAL/BluePrints/Game_Instance.Game_Instance_C|GetCurrent_Boat_Name (Variables|Default|GetGame%20Instance))))
    (Utilities|FlowControl|Delay 0.2)
    (CallFunction|PlayOneLetterAAT)))

(fn ConstructionScript
  (|CallParentFunction))